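; BP_CameraTrace is a mouse-driven trace actor that reports which object its line hits.
; Every tick it traces WorldDynamic objects from its own location to a point 300 units back along world X.
; The end point's Y and Z are the negated viewport mouse coordinates, used directly as world values without deprojection.
; It prints the hit actor's name and draws each trace as a persistent debug line.
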(event `self.ReceiveTick`
  (params (DeltaSeconds :type "Float (single-precision)"))
  (bind _returnvalue (`self.K2_GetActorLocation` self))
  (bind _returnvalue_2 (`WidgetLayoutLibrary.GetMousePositionOnViewport`))
  (bind _outhit (`KismetSystemLibrary.LineTraceSingleForObjects` :`Start` _returnvalue :`End` (`KismetMathLibrary.MakeVector` (+ (.x _returnvalue) -300.0) (* (`KismetMathLibrary.BreakVector2D` _returnvalue_2) -1.0) (* (`.Y` (`KismetMathLibrary.BreakVector2D` _returnvalue_2)) -1.0)) :`ObjectTypes` (`|MakeArray` "ObjectTypeQuery2" :!type "EObjectTypeQuery Enum") :`DrawDebugType` "Persistent"))
  (`KismetSystemLibrary.PrintString` (`KismetSystemLibrary.GetDisplayName` (`.HitActor` (`GameplayStatics.BreakHitResult` _outhit)))))

(fn `UserConstructionScript`)