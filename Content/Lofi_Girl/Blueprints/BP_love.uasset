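; BP_love is an actor that spawns the FXS_Loveshots effect when the player clicks the animated girl model.
; On BeginPlay it shows the mouse cursor and enables input on itself.
; Each left click traces under the cursor on the Visibility channel and matches the hit actor by its hard-coded display name.
; A match spawns the effect at the location of the SpawnLoc actor.
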(event `self.ReceiveBeginPlay`
  (bind _returnvalue (`GameplayStatics.GetPlayerControllerFromID` 0))
  (set `PlayerController.bShowMouseCursor` true _returnvalue)
  (`self.EnableInput` _returnvalue))

(event `Key|LeftMouseButton`
  (params (Key :type "Key Structure"))
  (:`Pressed`
    (if (`KismetStringLibrary.EqualEqual_StrStr` (`KismetSystemLibrary.GetDisplayName` (`.HitActor` (`GameplayStatics.BreakHitResult` (`PlayerController.GetHitResultUnderCursorByChannel` (`GameplayStatics.GetPlayerControllerFromID` 0) "TraceTypeQuery1" true)))) "maximoAnimationWithgirlModel_Anim_mixamo_com")
      (`NiagaraFunctionLibrary.SpawnSystemAtLocation` "/Game/Lofi_Girl/FX/FXS_Loveshots.FXS_Loveshots" (`self.K2_GetActorLocation` (`self.SpawnLoc`))))))

(fn `UserConstructionScript`)